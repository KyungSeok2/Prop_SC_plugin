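; Playable prop pawn for Propnight: a survivor's disguise form, driven as a physics-simulated static mesh with force movement, impulse jump and spring-arm camera.
; Left click traces from the camera and copies the mesh and material of "prop"-tagged actors; right click re-possesses the stored survivor.
; Possession toggles visibility, physics and collision.
; Req/Res event pairs relay these changes between server and clients, including the mesh transform sent every Tick.
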(event `InputAction|Jump`
  (params (Key :type "Key Structure"))
  ;[1 1 1 1 70] 점프
  (:`Pressed`
    (if (`self.IsGround`)
      (set `self.IsGround` false)
      (`PrimitiveComponent.AddImpulseAtLocation` (`self.Static Mesh`) (0.0 0.0 30000.0) (`SceneComponent.K2_GetComponentLocation` (`self.Static Mesh`)) "None")))
  (:`Released`
    (set `self.IsGround` false)))

(event `res_beginplay`
  (params (NewParam :type "/SurvivorCharacter_plugin/Propnight/GameMode/PlayLevel/BP_SurvivorCharacter Object Reference"))
  ;[1 1 1 1 70] 스폰이벤트
  (`SceneComponent.K2_AttachToComponent` (`self.Arrow`) (`self.Static Mesh`) "None" "KeepWorld" "KeepWorld" "KeepWorld" false))

(event `req_beginplay`
  (params (NewParam :type "/SurvivorCharacter_plugin/Propnight/GameMode/PlayLevel/BP_SurvivorCharacter Object Reference"))
  ;[1 1 1 1 70] 스폰이벤트
  ;;[1 0 0] 코멘트
  (`self.res_beginplay` NewParam))

(event `self.ReceiveBeginPlay`
  ;[1 1 1 1 70] 스폰이벤트
  ;;[1 1 1] 코멘트
  (bind _asbp_survivor_character (cast `/SurvivorCharacter_plugin/Propnight/GameMode/PlayLevel/BP_SurvivorCharacter` (`GameplayStatics.GetPlayerCharacter` 0)))
  (set `self.My Survivor Character` _asbp_survivor_character)
  (`self.req_beginplay` null))

(event `self.Static Mesh.OnComponentHit`
  (params (HitComponent :type "PrimitiveComponent Object Reference") (OtherActor :type "Actor Object Reference") (OtherComp :type "PrimitiveComponent Object Reference") (NormalImpulse :type "Vector Structure") (Hit :type "HitResult Structure (by ref)"))
  ;[1 1 1 1 70] 점프
)

(event `Key|One`
  (params (Key :type "Key Structure"))
  (bind _my_survivor_character (`self.My Survivor Character`))
  (:`Pressed`
    (`KismetSystemLibrary.PrintString` (`KismetStringLibrary.Concat_StrStr` (`KismetSystemLibrary.GetObjectName` (`self.GetOwner` _my_survivor_character)) (`KismetSystemLibrary.GetObjectName` _my_survivor_character)))))

(event `req_Server Loc Rot`
  (params (`Right Axis` :type "StaticMeshComponent Object Reference") (NewParam :type "Vector Structure") (NewParam2 :type "Rotator Structure"))
  ;[1 1 1 1 70] 카메라 정리 / 서버에 캐릭터의 위치값 회전값 전달
  ;;[1 0 0] (서버->클라)
  (`self.res_Server Loc Rot` `Right Axis` NewParam NewParam2))

(event `res_Server Loc Rot`
  (params (NewParam :type "StaticMeshComponent Object Reference") (NewParam2 :type "Vector Structure") (NewParam3 :type "Rotator Structure"))
  ;[1 1 1 1 70] 카메라 정리 / 서버에 캐릭터의 위치값 회전값 전달
  ;;[1 1 1] 전달받은 위치값을 각 클라이언트에 업데이트
  (`SceneComponent.K2_SetWorldLocationAndRotation` NewParam NewParam2 NewParam3 false false))

(event `self.ReceiveTick`
  (params (DeltaSeconds :type "Float (single-precision)"))
  (bind _static_mesh (`self.Static Mesh`))
  ;[1 1 1 1 70] 카메라 정리 / 서버에 캐릭터의 위치값 회전값 전달
  (`SceneComponent.K2_AddRelativeRotation` (`self.SpringArm`) (`KismetMathLibrary.MakeRotator` 0.0 (`self.GetInputAxisKeyValue`) (`self.GetInputAxisKeyValue`)) false false)
  ;;[1 1 1] 서버에 캐릭터 위치값 전달
  (`self.req_Server Loc Rot` _static_mesh (`SceneComponent.K2_GetComponentLocation` _static_mesh) (`SceneComponent.K2_GetComponentRotation` _static_mesh)))

(event `Key|LeftMouseButton`
  (params (Key :type "Key Structure"))
  ;[1 1 1] 코멘트
  ;;[1 1 1 1 70] 다른 프롭으로 변신 (좌클릭)
  ;;;[1 1 1] 다른 프롭으로 변신(클라->서버)
  (:`Pressed`
    (`self.req_transform`)))

(event `res_transform`
  (params (`Static Mesh` :type "StaticMesh Object Reference") (`Material Interface` :type "MaterialInterface Object Reference"))
  ;[1 1 1] 코멘트
  ;;[1 1 1 1 70] 다른 프롭으로 변신 (좌클릭)
  ;;;[1 1 1] 서버에서 전달받은 스테틱매시, 머터리얼로 변경
  (`self.Set Static Mesh` `Static Mesh` `Material Interface`))

(event `req_transform`
  (bind _camera (`self.Camera`))
  (bind _returnvalue (`SceneComponent.K2_GetComponentLocation` _camera))
  (bind _returnvalue_2 (`SceneComponent.GetForwardVector` _camera))
  ;[1 1 1] 코멘트
  ;;[1 1 1 1 70] 다른 프롭으로 변신 (좌클릭)
  ;;;[1 0 0] 클라->서버)
  ;;;;[1 1 1] 카메라 보는 방향으로 라인트레이스 발사
  (bind _outhit (`KismetSystemLibrary.LineTraceSingle` :`Start` (+ _returnvalue (* _returnvalue_2 700)) :`End` (+ _returnvalue (* _returnvalue_2 1200)) :`TraceChannel` "TraceTypeQuery1" :`DrawDebugType` "ForDuration"))
  ;;;;[1 1 1] 대상이 Prop 태그를 가지고 있다면
  (`/Engine/EditorBlueprintResources/StandardMacros.IsValid` (`.HitActor` (`GameplayStatics.BreakHitResult` _outhit))
    (:`Is Valid`
      (if (`self.ActorHasTag` (`.HitActor` (`GameplayStatics.BreakHitResult` _outhit)) "prop")
        (bind _staticmesh (`StaticMeshComponent.StaticMesh` (`self.GetComponentByClass` (`.HitActor` (`GameplayStatics.BreakHitResult` _outhit)) "/Script/Engine.StaticMeshComponent")))
        ;;;;[1 1 1] 스테틱매시 컴포넌트를 추출해서 클라이언트에 전달
        (`self.res_transform` _staticmesh (`StaticMesh.GetMaterial` _staticmesh 0))))))

(event `커스텀이벤트_0`
  ;[1 1 1 1 70] 프랍_ 굴리기(폐기)
)

(event `req_Client Possess`
  ;[1 1 1] 코멘트
  ;;[1 1 1 1 70] 빙의 이벤트
  ;;;[1 0 0] (서버->클라)
  (`self.res_Client Possess`))

(event `self.ReceivePossessed`
  (params (NewController :type "Controller Object Reference"))
  ;[1 1 1] 코멘트
  ;;[1 1 1 1 70] 빙의 이벤트
  (`self.req_Client Possess`))

(event `res_Client Possess`
  (bind _static_mesh (`self.Static Mesh`))
  ;[1 1 1] 코멘트
  ;;[1 1 1 1 70] 빙의 이벤트
  ;;;[1 1 1] 보이기
  (`SceneComponent.SetVisibility` _static_mesh true false)
  (`PrimitiveComponent.SetCollisionEnabled` _static_mesh "QueryAndPhysics")
  (`PrimitiveComponent.SetSimulatePhysics` _static_mesh true)
  (`PrimitiveComponent.SetCollisionResponseToChannel` (`self.Static Mesh`) "ECC_Pawn" "ECR_Block"))

(event `InputAxis|MoveForward` :overrideparent false
  (params (AxisValue :type "Float (single-precision)"))
  ;[1 1 1 1 70] 이동 (WASD)
  (`PrimitiveComponent.AddForce` (`self.Static Mesh`) (* (`KismetMathLibrary.GetForwardVector` (`SceneComponent.RelativeRotation` (`self.SpringArm`))) (* AxisValue 1500.0)) "None" true))

(event `res_to_Human`)

(event `InputAxis|MoveRight` :overrideparent false
  (params (AxisValue :type "Float (single-precision)"))
  ;[1 1 1 1 70] 이동 (WASD)
  (`PrimitiveComponent.AddForce` (`self.Static Mesh`) (* (`KismetMathLibrary.GetRightVector` (`SceneComponent.RelativeRotation` (`self.SpringArm`))) (* AxisValue 1500.0)) "None" true))

(event `req_to_Human`
  (params (arrow :type "ArrowComponent Object Reference") (Yaw :type "Float (double-precision)"))
  ;[1 1 1] 코멘트
  ;;[1 1 1 1 70] 현재 캐릭터의 빙의를 풀고 원래 캐릭터로 빙의 (우클릭)
  ;;;[1 0 0] 서버에서 이벤트 실행
  (`SceneComponent.K2_SetWorldRotation` arrow (`KismetMathLibrary.MakeRotator` 0.0 0.0 Yaw) false false)
  (`self.res_to human_MyClient`))

(event `res_to human_MyClient`
  ;[1 1 1] 코멘트
  ;;[1 1 1 1 70] 현재 캐릭터의 빙의를 풀고 원래 캐릭터로 빙의 (우클릭)
  ;;;[1 1 1] (서버->클라)
  ;;;;[0 1 1] 빙의해제 -> 다른캐릭터에 빙의
  (`self.res_to human_Server` (`GameplayStatics.GetPlayerController` 0) (`self.My Survivor Character`)))

(event `res_to human_Server`
  (params (controller :type "Controller Object Reference") (`Survivor Character` :type "/SurvivorCharacter_plugin/Propnight/GameMode/PlayLevel/BP_SurvivorCharacter Object Reference"))
  ;[1 1 1] 코멘트
  ;;[1 1 1 1 70] 현재 캐릭터의 빙의를 풀고 원래 캐릭터로 빙의 (우클릭)
  ;;;[1 1 1] (서버->클라)
  ;;;;[0 1 1] 빙의해제 -> 다른캐릭터에 빙의
  (`Controller.Possess` controller `Survivor Character`))

(event `Key|RightMouseButton`
  (params (Key :type "Key Structure"))
  (bind _arrow (`self.Arrow`))
  (bind (_returnvalue_roll _returnvalue_pitch _returnvalue_yaw) (`KismetMathLibrary.BreakRotator` (`SceneComponent.K2_GetComponentRotation` (`self.Camera`))))
  ;[1 1 1] 코멘트
  ;;[1 1 1 1 70] 현재 캐릭터의 빙의를 풀고 원래 캐릭터로 빙의 (우클릭)
  ;;;[1 1 1] 변신 해제
  (:`Pressed`
    (`SceneComponent.K2_SetWorldRotation` _arrow (`KismetMathLibrary.MakeRotator` 0.0 0.0 _returnvalue_yaw) false false)
    (`self.req_to_Human` _arrow _returnvalue_yaw)))

(event `req_Client UnPossess`
  ;[1 1 1] 코멘트
  ;;[1 1 1 1 70] 빙의 풀렸을때 이벤트
  ;;;[1 0 0] (서버->클라)
  (`self.res_Client UnPossess`))

(event `res_Client UnPossess`
  (bind _static_mesh (`self.Static Mesh`))
  ;[1 1 1] 코멘트
  ;;[1 1 1 1 70] 빙의 풀렸을때 이벤트
  ;;;[1 1 1] 숨기기
  (`SceneComponent.SetVisibility` _static_mesh false false)
  (`PrimitiveComponent.SetSimulatePhysics` _static_mesh false)
  (`PrimitiveComponent.SetCollisionEnabled` _static_mesh "NoCollision")
  (`PrimitiveComponent.SetCollisionResponseToChannel` (`self.Static Mesh`) "ECC_Pawn" "ECR_Ignore"))

(event `self.ReceiveUnpossessed`
  (params (OldController :type "Controller Object Reference"))
  ;[1 1 1] 코멘트
  ;;[1 1 1 1 70] 빙의 풀렸을때 이벤트
  (`self.req_Client UnPossess`))

(event `Key|Q`
  (params (Key :type "Key Structure"))
  (bind _static_mesh (`self.Static Mesh`))
  (bind (_relativerotation_roll _relativerotation_pitch _relativerotation_yaw) (`KismetMathLibrary.BreakRotator` (`SceneComponent.RelativeRotation` _static_mesh)))
  ;[1 1 1 1 70] 위치 정렬 (Q키)
  (:`Pressed`
    (`SceneComponent.K2_SetRelativeRotation` _static_mesh (`KismetMathLibrary.MakeRotator` 0.0 0.0 _relativerotation_yaw) false false)))

(fn `Mesh Move`
  (params (A :type "Vector Structure") (A2 :type "Float (double-precision)")))

(fn `OnRep_Return Value Z (Yaw)`)

(fn `Set Static Mesh`
  (params (GetStaticMesh :type "StaticMesh Object Reference") (GetMaterial :type "MaterialInterface Object Reference") (SurvivorCharacter :type "Character Object Reference"))
  ;[1 1 1] SurvivorCharacter 혹은
  ; PropCharacter 에서
  ; 상호작용키(F) 누를때 함수 실행
  ;[1 1 1] 스테틱매시를 가져온다.
  (`StaticMeshComponent.SetStaticMesh` (`self.Static Mesh`) GetStaticMesh)
  (`PrimitiveComponent.SetMaterial` (`self.Static Mesh`) 0 GetMaterial)
  ;[1 1 1] 콜리젼켜진 상태가 아니라면
  ; SurvivorCharacter의 회전 값을 준다
  (if (not (`PrimitiveComponent.K2_IsCollisionEnabled` (`self.Static Mesh`)))
    (`SceneComponent.K2_SetRelativeRotation` (`self.SpringArm`) (`self.K2_GetActorRotation` SurvivorCharacter) false false)))

(fn `UserConstructionScript`)